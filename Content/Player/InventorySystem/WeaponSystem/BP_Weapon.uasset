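; BP_Weapon is a weapon Blueprint in the player's inventory weapon system, carrying a WeaponInfo struct that describes the weapon.
; The struct groups combat stats, ammo state, attachment sockets, animations and effect data.
; The Construction Script rebuilds WeaponInfo with the actor's own class in its first field, copying every other field unchanged.
; The event graph holds only disabled default events, so this Blueprint runs no gameplay logic.
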(event EventBeginPlay
  (|CallParentFunction) ; 此节点被禁用，将不会被调用。\n从引脚连出引线来编译功能。
)

(event Collision|EventActorBeginOverlap
  (params (OtherActor :type Actor%20Object%20Reference))
  (|CallParentFunction OtherActor) ; 此节点被禁用，将不会被调用。\n从引脚连出引线来编译功能。
)

(event EventTick
  (params (DeltaSeconds :type Float%20%28single-precision%29))
  (|CallParentFunction DeltaSeconds) ; 此节点被禁用，将不会被调用。\n从引脚连出引线来编译功能。
)

(fn ConstructionScript
  (|CallParentFunction)
  (Variables|Default|SetWeaponInfo (Utilities|Struct|MakeS_WeaponInfo (Utilities|GetClass self) (.type (Variables|Default|GetWeaponInfo)) (.开火动画序列 (Variables|Default|GetWeaponInfo)) (.战斗插槽 (Variables|Default|GetWeaponInfo)) (.挂载插槽1 (Variables|Default|GetWeaponInfo)) (.挂载插槽2 (Variables|Default|GetWeaponInfo)) (.射击距离 (Variables|Default|GetWeaponInfo)) (.开火速度 (Variables|Default|GetWeaponInfo)) (.damage (Variables|Default|GetWeaponInfo)) (.备用弹夹子弹数量 (Variables|Default|GetWeaponInfo)) (.当前载弹量 (Variables|Default|GetWeaponInfo)) (.弹夹载弹量 (Variables|Default|GetWeaponInfo)) (.后坐力偏移量 (Variables|Default|GetWeaponInfo)) (.使用弹药类型 (Variables|Default|GetWeaponInfo)) (.射击类型 (Variables|Default|GetWeaponInfo)) (.弹道类型 (Variables|Default|GetWeaponInfo)) (.切换武器蒙太奇人物用 (Variables|Default|GetWeaponInfo)) (.武器装弹动画序列武器用 (Variables|Default|GetWeaponInfo)) (.人物装弹蒙太奇人物用 (Variables|Default|GetWeaponInfo)) (.开火蒙太奇人物用 (Variables|Default|GetWeaponInfo)) (.ammoinfo (Variables|Default|GetWeaponInfo)) (.effectinfo (Variables|Default|GetWeaponInfo)))))