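; BP_ItemBase is an inventory item actor that builds its visual from the item ID in its SlotItemInfo.
; The construction script looks up the mesh type, then adds and stores either a static mesh component, with physics simulation off, or a skeletal mesh component.
; 物品描边 toggles Render Custom Depth on the matching mesh for outlining.
; The event graph holds no logic.
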(event EventBeginPlay)

(event Collision|EventActorBeginOverlap
  (params (OtherActor :type Actor%20Object%20Reference)))

(event EventTick
  (params (DeltaSeconds :type Float%20%28single-precision%29)))

(fn ConstructionScript
  (bind _slotiteminfo (Variables|Default|GetSlotItemInfo))
  (bind _物品id (Utilities|Struct|BreakS_SlotInfo _slotiteminfo))
  (switch Utilities|FlowControl|Switch|SwitchonMeshType (CallFunction|获得物品mesh类型 _物品id)
    (:NewEnumerator0
      (bind _returnvalue (AddComponent|AddStaticMeshComponent false))
      (Physics|SetSimulatePhysics _returnvalue false)
      (Components|StaticMesh|SetStaticMesh _returnvalue (CallFunction|获得物品静态mesh _物品id))
      (Variables|Default|SetItemStaticMesh _returnvalue))
    (:NewEnumerator1
      (bind _returnvalue_2 (AddComponent|AddSkeletalMeshComponent false))
      (Class|SkinnedMeshComponent|SetSkeletalMesh _returnvalue_2 (CallFunction|获得物品骨骼mesh _物品id) true)
      (Variables|Default|SetItemSkeletalMesh _returnvalue_2))))

(fn 物品描边
  (params (是否开启描边 :type Boolean))
  (switch Utilities|FlowControl|Switch|SwitchonMeshType (CallFunction|获得物品mesh类型 (Utilities|Struct|BreakS_SlotInfo (Variables|Default|GetSlotItemInfo)))
    (:NewEnumerator0
      (Rendering|SetRenderCustomDepth (Variables|Default|GetItemStaticMesh) 是否开启描边))
    (:NewEnumerator1
      (Rendering|SetRenderCustomDepth (Variables|Default|GetItemSkeletalMesh) 是否开启描边))))