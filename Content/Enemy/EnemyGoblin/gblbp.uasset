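; Goblin enemy Blueprint that tracks health, reacts to damage and handles its own death.
; On spawn it picks a random skin, giving the MI_EnemyGoblin_02 variant its own health and damage, and fills its attack montage array.
; Damage lowers HP, plays a hit montage and reports a damage event; Tick handles death by disabling collision, detaching the controller and destroying the actor after a delay.
; A player-bound event keeps the health bar facing the camera.
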(event Custom|AI_StateBarRotation
  (bind _returnvalue (Game|GetPlayerCameraManager 0))
  (bind _hp_bar (Variables|Default|GetHP_Bar))
  (bind _hp_bar_2 (Variables|Default|GetHP_Bar))
  (bind _returnvalue_2 (Transformation|GetActorLocation _returnvalue))
  (bind _returnvalue_3 (Transformation|GetWorldLocation _hp_bar_2))
  (bind _returnvalue_4 (Math|Rotator|FindLookatRotation _returnvalue_3 _returnvalue_2))
  ;[1 1 1] 使状态条一直朝向玩家
  (Utilities|IsValid _hp_bar
    (:Is%20Valid
      (Transformation|SetWorldRotation _hp_bar (Math|Rotator|MakeRotator (.roll _returnvalue_4) 0.0 (.yaw _returnvalue_4)) false false))))

(event EventBeginPlay
  (Utilities|FlowControl|Sequence
    (:then_0
      (Variables|Default|Set已死亡 false)
      (Variables|Default|SetCurrentHP (Variables|Default|GetAI%20Health)))
    (:then_1
      (bind _asplayer (Utilities|Casting|CastToPLayer (Game|GetPlayerCharacter 0)))
      (Variables|Default|SetAs%20PLayer _asplayer))
    (:then_2
      ;[1 1 1] 使状态条一直朝向玩家
      (bind _asai_health_bar (Utilities|Casting|CastToAI_HealthBar (UserInterface|GetUserWidgetObject (Variables|Default|GetHP_Bar))))
      (Variables|/Game/Enemy/AI_HealthBar.AI_HealthBar_C|SetAI _asai_health_bar self)
      (EventDispatchers|BindEventtoStateBarRotation (Variables|Default|GetAs%20PLayer) (delegate Custom|AI_StateBarRotation)))
    (:then_3
      (CallFunction|刷新随机材质种类怪物)
      (CallFunction|更新攻击蒙太奇动画数组))))

(event EventTakeDamage
  (params (命中结果 :type Hit%20Result%20Structure) (伤害值 :type Float%20%28single-precision%29)))

(event EventTick
  (params (DeltaSeconds :type Float%20%28single-precision%29))
  (bind _hp_bar (Variables|Default|GetHP_Bar))
  (bind _mesh (Variables|Character|GetMesh))
  (bind _returnvalue (Components|SkeletalMesh|GetAnimInstance _mesh))
  (Utilities|FlowControl|Sequence
    (:then_0
      (if (<= (Variables|Default|GetCurrentHP) 0.0)
        (Variables|Default|Set已死亡 true)
        (Animation|Montage|MontageStop _returnvalue 0.0 (Animation|Montage|GetCurrentActiveMontage _returnvalue))
        (Collision|SetCollisionEnabled (Variables|Collision|GetCapsuleComponent) "NoCollision")
        (Class|Pawn|DetachfromControllerPendingDestroy)
        (Utilities|IsValid _hp_bar
          (:Is%20Valid
            (Components|DestroyComponent _hp_bar)
            (Utilities|FlowControl|DoOnce false
              (:Completed
                (Utilities|FlowControl|Delay 5.0)
                (Actor|DestroyActor)))))))))

(event Game|Damage|EventAnyDamage
  (params (Damage :type Float%20%28single-precision%29) (DamageType :type Damage%20Type%20Object%20Reference) (InstigatedBy :type Controller%20Object%20Reference) (DamageCauser :type Actor%20Object%20Reference))
  (Class|AISenseDamage|ReportDamageEvent self DamageCauser Damage "0, 0, 0" "0, 0, 0" "damage")
  (Variables|Default|SetCurrentHP (- (Variables|Default|GetCurrentHP) Damage))
  (Animation|Montage|MontagePlay (Components|SkeletalMesh|GetAnimInstance (Variables|Character|GetMesh)) "/Game/Enemy/EnemyGoblin/Animations/蒙太奇/Anim_Hit_Montage.Anim_Hit_Montage" 0.3 "Duration" 0.0 true))

(event EventTakeRadiusDamage
  (params (命中结果 :type Hit%20Result%20Structure) (AmmoInfo :type S%20Ammo%20Info%20Structure)))

(fn ConstructionScript)

(fn 刷新随机材质种类怪物
  (bind _mesh (Variables|Character|GetMesh))
  (Rendering|Material|SetMaterial _mesh 0 (.OutItem (Utilities|Array|Random (Variables|Default|Get种类))))
  (if (Utilities|Enum|Equal(Enum) (Utilities|GetDisplayName (Rendering|Material|GetMaterial _mesh 0)) "MI_EnemyGoblin_02")
    (bind _output_get (Variables|Default|SetAI%20Health 3e+02))
    (Variables|Default|SetCurrentHP _output_get)
    (Variables|Default|SetBaseDamage 1e+01)))

(fn 更新攻击蒙太奇动画数组
  (bind _攻击动画蒙太奇 (Variables|Default|Get攻击动画蒙太奇))
  (Utilities|Array|Add _攻击动画蒙太奇 "/Game/Enemy/EnemyGoblin/Animations/蒙太奇/Anim_Attack1_Montage.Anim_Attack1_Montage")
  (Utilities|Array|Add _攻击动画蒙太奇 "/Game/Enemy/EnemyGoblin/Animations/蒙太奇/Anim_Attack2_Montage.Anim_Attack2_Montage"))