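; Zombie enemy Blueprint that handles taking damage and holds its attack animation montages.
; On AnyDamage it reports a damage event with the causer as instigator, subtracts the damage from CurrentHP and plays a sped-up hit montage.
; A separate function, 更新攻击蒙太奇动画数组, adds two attack montages to an array; no caller or death handling appears here.
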(event EventBeginPlay
  (|CallParentFunction) ; 此节点被禁用，将不会被调用。\n从引脚连出引线来编译功能。
)

(event Collision|EventActorBeginOverlap
  (params (OtherActor :type Actor%20Object%20Reference)))

(event EventTick
  (params (DeltaSeconds :type Float%20%28single-precision%29))
  (|CallParentFunction DeltaSeconds) ; 此节点被禁用，将不会被调用。\n从引脚连出引线来编译功能。
)

(event Game|Damage|EventAnyDamage
  (params (Damage :type Float%20%28single-precision%29) (DamageType :type Damage%20Type%20Object%20Reference) (InstigatedBy :type Controller%20Object%20Reference) (DamageCauser :type Actor%20Object%20Reference))
  (Class|AISenseDamage|ReportDamageEvent self DamageCauser 0.0 "0, 0, 0" "0, 0, 0" "damage")
  (Variables|Default|SetCurrentHP (- (Variables|Default|GetCurrentHP) Damage))
  (Animation|Montage|MontagePlay (Components|SkeletalMesh|GetAnimInstance (Variables|Character|GetMesh)) "/Game/Enemy/Zombie/Animations/蒙太奇/Zombie_Anim_Hit_Montage.Zombie_Anim_Hit_Montage" 1.25 "Duration" 0.0 true))

(fn ConstructionScript
  (|CallParentFunction))

(fn 更新攻击蒙太奇动画数组
  (bind _攻击动画蒙太奇 (Variables|Default|Get攻击动画蒙太奇))
  (Utilities|Array|Add _攻击动画蒙太奇 "/Game/Enemy/Zombie/Animations/蒙太奇/Zombie_Anim_Attack1_Montage.Zombie_Anim_Attack1_Montage")
  (Utilities|Array|Add _攻击动画蒙太奇 "/Game/Enemy/Zombie/Animations/蒙太奇/Zombie_Anim_Attack2_Montage.Zombie_Anim_Attack2_Montage"))