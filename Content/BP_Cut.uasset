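; BP_Cut is an actor that can be sliced at runtime into physical pieces along a given plane.
; Its construction script copies the chosen static mesh into a ProceduralMesh with collision, then destroys the static mesh component.
; The CUT_EVETN event slices that mesh at the supplied position and normal, capping the cut with a new material section.
; The other half is created, set to simulate physics and pushed away with a fixed velocity-change impulse.
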(event Custom|CUT_EVETN
  (params (PlanePosition :type Vector) (PlaneNormal :type Vector))
  (bind _outotherhalfprocmesh (Class|KismetProceduralMeshLibrary|SliceProceduralMesh (Variables|Default|GetProceduralMesh) PlanePosition PlaneNormal true "CreateNewSectionForCap" "/Game/AK47/AK_Inst.AK_Inst"))
  (Physics|SetSimulatePhysics _outotherhalfprocmesh true)
  (Physics|AddImpulse _outotherhalfprocmesh "100.000000,100.000000,100.000000" "None" true))

(event EventBeginPlay)

(event Collision|EventActorBeginOverlap
  (params (OtherActor :type Actor%20Object%20Reference)))

(event EventTick
  (params (DeltaSeconds :type Float%20%28single-precision%29)))

(fn ConstructionScript
  (bind _staticmesh (Variables|Default|GetStaticMesh))
  (Components|StaticMesh|SetStaticMesh (Variables|Default|GetStaticMesh) (Variables|Default|GetMesh))
  (Class|KismetProceduralMeshLibrary|CopyProceduralMeshfromStaticMeshComponent _staticmesh 0 (Variables|Default|GetProceduralMesh) true)
  (Components|DestroyComponent _staticmesh))